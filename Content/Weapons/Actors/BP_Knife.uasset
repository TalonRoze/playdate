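; BP_Knife is a melee weapon actor that damages BP_EnemyBase enemies through a box hitbox.
; The box has collision off from BeginPlay, and AttackKnife switches it to query-only for a brief delay before disabling it again.
; Overlaps during that window apply KnifeDamage to the enemy, crediting the controller of the owning BP_FirstPersonCharacter as instigator.
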(event `self.ReceiveBeginPlay`
  ; Turn off collision at the start
  (`PrimitiveComponent.SetCollisionEnabled` (`self.Box`) "NoCollision"))

(event `AttackKnife`
  (`PrimitiveComponent.SetCollisionEnabled` (`self.Box`) "QueryOnly")
  (`KismetSystemLibrary.Delay` 0.1)
  (`PrimitiveComponent.SetCollisionEnabled` (`self.Box`) "NoCollision"))

(event `self.Box.OnComponentBeginOverlap`
  (params (OverlappedComponent :type "PrimitiveComponent Object Reference") (OtherActor :type "Actor Object Reference") (OtherComp :type "PrimitiveComponent Object Reference") (OtherBodyIndex :type Integer) (bFromSweep :type Boolean) (SweepResult :type "HitResult Structure (by ref)"))
  ; Deal Damage
  (bind _asbp_enemy_base (cast `/Game/FirstPerson/Blueprints/Enemies/BP_EnemyBase` OtherActor))
  (bind _asbp_first_person_character (cast `/Game/FirstPerson/Blueprints/BP_FirstPersonCharacter` (`self.GetOwner`)))
  (`GameplayStatics.ApplyDamage` _asbp_enemy_base (`self.Knife_Damage`) (`Pawn.GetController` _asbp_first_person_character) self))

(fn `UserConstructionScript`)