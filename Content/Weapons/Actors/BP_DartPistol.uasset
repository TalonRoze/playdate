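; BP_DartPistol is the pistol's dart projectile, which damages enemies and leaves a pickup where it ends up.
; A capsule overlap with a BP_EnemyBase applies the pistol dart damage, credited to the first player controller.
; Both that hit and the DartMovement projectile stopping destroy the dart and spawn a BP_PickupDartPistol at its transform.
; Overlaps with any other actor type are ignored.
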(event `self.Capsule.OnComponentBeginOverlap`
  (params (OverlappedComponent :type "PrimitiveComponent Object Reference") (OtherActor :type "Actor Object Reference") (OtherComp :type "PrimitiveComponent Object Reference") (OtherBodyIndex :type Integer) (bFromSweep :type Boolean) (SweepResult :type "HitResult Structure (by ref)"))
  ; Deal Damage
  (bind _asbp_enemy_base (cast `/Game/FirstPerson/Blueprints/Enemies/BP_EnemyBase` OtherActor))
  (`GameplayStatics.ApplyDamage` _asbp_enemy_base (`self.Dart Damage Pistol`) (`GameplayStatics.GetPlayerController` 0) self)
  (`self.K2_DestroyActor`)
  (`|SpawnActorFromClass` "/Game/Weapons/Actors/BP_PickupDartPistol.BP_PickupDartPistol_C" (`self.GetTransform`) "AlwaysSpawn" "MultiplyWithRoot" null (`self.GetInstigator`)))

(event `self.DartMovement.OnProjectileStop`
  (params (ImpactResult :type "HitResult Structure (by ref)"))
  ; Deal Damage
  (`self.K2_DestroyActor`)
  (`|SpawnActorFromClass` "/Game/Weapons/Actors/BP_PickupDartPistol.BP_PickupDartPistol_C" (`self.GetTransform`) "AlwaysSpawn" "MultiplyWithRoot" null (`self.GetInstigator`)))

(fn `UserConstructionScript`)