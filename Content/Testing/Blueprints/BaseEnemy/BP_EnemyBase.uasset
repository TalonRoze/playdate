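; BP_EnemyBase is a test base enemy with health, a toy hammer and leashed chase AI.
; Pawn sensing triggers chasing the player with a timeline-driven hammer swing, or returning to start once beyond MaxFollowDistance.
; Player overlap with its hitbox damages the enemy itself as a test.
; At zero health it spawns placeholder effects, destroys itself and prints its score value, without awarding it.
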(event `self.ReceiveAnyDamage`
  (params (Damage :type "Float (single-precision)") (DamageType :type "DamageType Object Reference") (InstigatedBy :type "Controller Object Reference") (DamageCauser :type "Actor Object Reference"))
  ; Subtract Health on Damage
  (bind _output_get (set `self.CurrentHealth` (`KismetMathLibrary.FTrunc` (- (`self.CurrentHealth`) Damage))))
  ; Check health, <= 0 health = death
  (if (<= _output_get 0)
    (`self.HandleDeath`)))

(event `HandleDeath`
  (bind _returnvalue (`self.K2_GetActorLocation`))
  ;[1 0.15 0.15 0.5] HandleDeath, need to add score
  (`GameplayStatics.SpawnEmitterAtLocation` "/Engine/Tutorial/SubEditors/TutorialAssets/TutorialParticleSystem.TutorialParticleSystem" _returnvalue)
  (`GameplayStatics.PlaySoundAtLocation` "/Engine/EngineSounds/1kSineTonePing.1kSineTonePing" _returnvalue (struct) 1.0 1.0 0.0 null null null null)
  (`self.K2_DestroyActor`)
  (`KismetSystemLibrary.PrintString` (`KismetStringLibrary.Concat_StrStr` (`KismetSystemLibrary.GetDisplayName` self) " has died. score: " (`KismetStringLibrary.Conv_IntToString` (`self.ScoreValue`))) true true (struct :`R` 1.0 :`A` 1.0)))

(event `self.ReceiveBeginPlay`
  ; Initialise health
  (set `self.CurrentHealth` (`self.MaxHealth`))
  (set `self.StartingLocation` (`self.K2_GetActorLocation`)))

(event `self.Hitbox.OnComponentBeginOverlap`
  (params (OverlappedComponent :type "PrimitiveComponent Object Reference") (OtherActor :type "Actor Object Reference") (OtherComp :type "PrimitiveComponent Object Reference") (OtherBodyIndex :type Integer) (bFromSweep :type Boolean) (SweepResult :type "HitResult Structure (by ref)"))
  ; Damage test, when overlapping with player
  (bind _asbp_first_person_character (cast `/Game/FirstPerson/Blueprints/BP_FirstPersonCharacter` OtherActor))
  (`GameplayStatics.ApplyDamage` self (`KismetMathLibrary.Abs` 1.0) (`self.GetController` _asbp_first_person_character) OtherActor)
  (`KismetSystemLibrary.PrintString` (`KismetStringLibrary.Concat_StrStr` (`KismetSystemLibrary.GetDisplayName` self) " hit. remaining health: " (`KismetStringLibrary.Conv_IntToString` (`self.CurrentHealth`))) true true (struct :`R` 1.0 :`A` 1.0)))

(event `FollowPawn`
  ;[0.4616 0.04184 0.6319 0.5] AI
  (`|AIMoveTo` self (0.0 0.0 0.0) (`GameplayStatics.GetPlayerCharacter` 0)))

(event `self.PawnSensing.OnSeePawn`
  (params (Pawn :type "Pawn Object Reference"))
  ;[0.4616 0.04184 0.6319 0.5] AI
  ;;[1 0.7859 0 0.5] Makes enemy go back to their starting location when too far from their spot
  (if (> (`KismetMathLibrary.Vector_Distance` (`self.K2_GetActorLocation`) (`self.StartingLocation`)) (`self.MaxFollowDistance`))
    (`self.GoBackToStart`)
    (bind (_direction _hammerswing) (`Timeline|HammerSwing` :!via `Stop` :!label _label)
      (:`Update`
        (`SceneComponent.K2_SetRelativeRotation` (`self.Toy_Hammer`) (`KismetMathLibrary.MakeRotator` 0.0 (* _hammerswing (`KismetMathLibrary.Abs` 90.0))) false false)))
    (else
      (`self.FollowPawn`)
      (goto _label))))

(event `GoBackToStart`
  ;[0.4616 0.04184 0.6319 0.5] AI
  (`|AIMoveTo` self (`self.StartingLocation`) null))

(fn `UserConstructionScript`)